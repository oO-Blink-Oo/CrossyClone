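; BP_Player is a player Blueprint that handles basic movement and creates the on-screen Crossy widget at BeginPlay.
; MoveForward and MoveRight axes feed movement input along the actor's forward and right vectors, scaled by MaxSpeed.
; Tick consumes that input and applies it, scaled by delta time, as an unswept local offset.
; The world-space vectors are applied in local space, so actor rotation affects direction twice.
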(event `InputAxis|MoveForward`
  (params (AxisValue :type "Float (single-precision)"))
  ;[1 1 1] MoveForward/Backward
  (`self.AddMovementInput` (`self.GetActorForwardVector`) (* AxisValue (`self.MaxSpeed`))))

(event `InputAxis|MoveRight`
  (params (AxisValue :type "Float (single-precision)"))
  ;[1 1 1] MoveRight/Left
  (`self.AddMovementInput` (`self.GetActorRightVector`) (* AxisValue (`self.MaxSpeed`))))

(event `self.ReceiveBeginPlay`
  (bind _returnvalue (`|CreateWidget` "/Game/UI/Crossy.Crossy_C"))
  (`UserWidget.AddToViewport` _returnvalue 0))

(event `self.ReceiveTick`
  (params (DeltaSeconds :type "Float (single-precision)"))
  (bind _returnvalue (`self.ConsumeMovementInputVector`))
  (`self.K2_AddActorLocalOffset` (* _returnvalue DeltaSeconds)))

(fn `UserConstructionScript`)